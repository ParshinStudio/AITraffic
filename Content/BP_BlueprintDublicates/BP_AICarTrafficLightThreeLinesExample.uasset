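; Traffic light Blueprint for AI cars, apparently an example three-lane variant, that adds a fourth set of red, yellow and green lamps to its parent.
; Overridden SwitchMainLights calls the parent, then shows the fourth green lamp on Green and the red one on Red, Pedestrians or Delay.
; Overridden SwitchYellowLight calls the parent, then toggles the fourth yellow lamp's visibility.
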(event EventSwitchMainLights
  (params (NewLightState :type ELightState%20Enum :default "NewEnumerator0"))
  (bind _redlightfourth (Variables|Default|GetRedLightFourth))
  (bind _greenlightfourth (Variables|Default|GetGreenLightFourth))
  (|CallParentFunction NewLightState)
  (switch Utilities|FlowControl|Switch|SwitchonELightState NewLightState
    (:NewEnumerator0
      (Rendering|SetVisibility _greenlightfourth true false)
      (Rendering|SetVisibility _redlightfourth false false))
    (:NewEnumerator1
      (Rendering|SetVisibility _greenlightfourth false false :!label _label)
      (Rendering|SetVisibility _redlightfourth true false))
    (:NewEnumerator2
      (goto _label))
    (:NewEnumerator3
      (goto _label))))

(event EventSwitchYellowLight
  (params (SwitchOn :type Boolean))
  (|CallParentFunction SwitchOn)
  (Rendering|SetVisibility (Variables|Default|GetYellowLightFourth) SwitchOn false))

(fn ConstructionScript)