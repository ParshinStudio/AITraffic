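; An example AI car traffic light Blueprint that extends a parent traffic light with an additional "Third" set of green, red and yellow lights.
; It overrides the main and yellow switch events, calls the parent, then toggles visibility on the third set.
; The third green shows only in the Green state, while Red, Pedestrians and Delay all show red.
; Yellow follows the switch flag independently.
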(event EventSwitchMainLights
  (params (NewLightState :type ELightState%20Enum :default "NewEnumerator0"))
  (bind _greenlightthird (Variables|Default|GetGreenLightThird))
  (bind _redlightthird (Variables|Default|GetRedLightThird))
  (|CallParentFunction NewLightState)
  (switch Utilities|FlowControl|Switch|SwitchonELightState NewLightState
    (:NewEnumerator0
      (Rendering|SetVisibility _greenlightthird true false)
      (Rendering|SetVisibility _redlightthird false false))
    (:NewEnumerator1
      (Rendering|SetVisibility _greenlightthird false false :!label _label)
      (Rendering|SetVisibility _redlightthird true false))
    (:NewEnumerator2
      (goto _label))
    (:NewEnumerator3
      (goto _label))))

(event EventSwitchYellowLight
  (params (SwitchOn :type Boolean))
  (|CallParentFunction SwitchOn)
  (Rendering|SetVisibility (Variables|Default|GetYellowLightThird) SwitchOn false))

(fn ConstructionScript)