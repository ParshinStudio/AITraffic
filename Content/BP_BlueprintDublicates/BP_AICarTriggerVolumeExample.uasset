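; Multi-purpose trigger volume that directs BP_AICarExample traffic, with behavior selected by TriggerType.
; On overlap it gates cars at traffic lights, flags crossroads, switches splines, randomly diverts cars into parking, stops them in slots or destroys them.
; SetLetPassCrossRoads updates the stored waiting car, while parking occupancy clears on departure or by timer.
; End overlap checks Traffic Light twice, so its Cross Road reset is unreachable.
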(event OnComponentBeginOverlap(TriggerVolume)
  (params (OverlappedComponent :type Primitive%20Component%20Object%20Reference) (OtherActor :type Actor%20Object%20Reference) (OtherComp :type Primitive%20Component%20Object%20Reference) (OtherBodyIndex :type Integer) (bFromSweep :type Boolean) (SweepResult :type Hit%20Result%20Structure%20%28by%20ref%29))
  (bind _asbp_aicar_example (Utilities|Casting|CastToBP_AICarExample OtherActor))
  (switch Utilities|FlowControl|Switch|SwitchonETriggerType (Variables|AIConfig|GetTriggerType)
    (:NewEnumerator0
      (bind _output_get (Variables|TriggerBoxVars|SetTriggeredCar _asbp_aicar_example))
      (Variables|/Game/BP_BlueprintDublicates/BP_AICarExample.BP_AICarExample_C|SetCanMove _asbp_aicar_example (Variables|TriggerBoxVars|GetLetPassCrossRoads))
      (Default|ChooseNewSplineonCrossroad _output_get (Variables|AIConfig|GetNewSplines))
      (Variables|/Game/BP_BlueprintDublicates/BP_AICarExample.BP_AICarExample_C|SetGreenLightTime _asbp_aicar_example (Variables|TriggerBoxVars|GetGreenLightTimer))
      (Variables|/Game/BP_BlueprintDublicates/BP_AICarExample.BP_AICarExample_C|SetIsOnMainDirection _asbp_aicar_example (Variables|TriggerBoxVars|GetIsMainDirection))
      (if (Variables|TriggerBoxVars|GetLetPassCrossRoads)
        (Variables|TriggerBoxVars|SetTriggeredCar 0)))
    (:NewEnumerator1
      (Default|SetNewSpline _asbp_aicar_example (Utilities|Array|Get(acopy) (Variables|AIConfig|GetNewSplines))))
    (:NewEnumerator2
      (Variables|/Game/BP_BlueprintDublicates/BP_AICarExample.BP_AICarExample_C|SetIsOnCrossRoad _asbp_aicar_example true)
      (Variables|/Game/BP_BlueprintDublicates/BP_AICarExample.BP_AICarExample_C|SetStartLeftTurnRotation _asbp_aicar_example (Transformation|GetActorRotation _asbp_aicar_example)))
    (:NewEnumerator3
      (if (Math|Boolean|ANDBoolean (Variables|AIConfig|GetBoxTriggerParking) (not (Variables|/Game/BP_BlueprintDublicates/BP_AICarExample.BP_AICarExample_C|GetMoving _asbp_aicar_example)) (not (Variables|TriggerBoxVars|GetOccupied)) (< (Math|Random|RandomFloatinRange 0.0 1e+02) 2e+01))
        (Variables|TriggerBoxVars|SetOldSpline (Variables|/Game/BP_BlueprintDublicates/BP_AICarExample.BP_AICarExample_C|GetCurrentSpline _asbp_aicar_example))
        (Default|SetNewSpline _asbp_aicar_example (Utilities|Array|Get(acopy) (Variables|AIConfig|GetNewSplines)))
        (Variables|TriggerBoxVars|SetOccupied true)
        (elif (Math|Boolean|ANDBoolean (Variables|AIConfig|GetBoxTriggerParking) (Variables|/Game/BP_BlueprintDublicates/BP_AICarExample.BP_AICarExample_C|GetMoving _asbp_aicar_example) (Variables|TriggerBoxVars|GetOccupied))
          (Default|StopLeaveParkingSlot _asbp_aicar_example (Variables|TriggerBoxVars|GetOldSpline))
          (Variables|TriggerBoxVars|SetOccupied false)
          (elif (Math|Boolean|ANDBoolean (not (Variables|AIConfig|GetBoxTriggerParking)) (not (Variables|TriggerBoxVars|GetOccupied)) (< (Math|Random|RandomFloatinRange 0.0 1e+02) 2e+01))
            (Default|SetNewSpline _asbp_aicar_example (Utilities|Array|Get(acopy) (Variables|AIConfig|GetNewSplines)))
            (Variables|TriggerBoxVars|SetOccupied true)
            (Utilities|Time|SetTimerbyFunctionName self "ResetOccupied" 1.0 false (+ (Variables|/Game/BP_BlueprintDublicates/BP_AICarExample.BP_AICarExample_C|GetLeaveParkingSlotTimer _asbp_aicar_example) 5.0))))))
    (:NewEnumerator4
      (Default|StopinParkingSlot _asbp_aicar_example (Variables|AIConfig|GetBoxParking)))
    (:NewEnumerator5
      (Actor|DestroyActor _asbp_aicar_example))))

(event OnComponentEndOverlap(TriggerVolume)
  (params (OverlappedComponent :type Primitive%20Component%20Object%20Reference) (OtherActor :type Actor%20Object%20Reference) (OtherComp :type Primitive%20Component%20Object%20Reference) (OtherBodyIndex :type Integer))
  (bind _triggertype (Variables|AIConfig|GetTriggerType))
  (if (or (Utilities|Enum|Equal(Enum) _triggertype "NewEnumerator0") (Utilities|Enum|Equal(Enum) _triggertype "NewEnumerator0"))
    (bind _asbp_aicar_example (Utilities|Casting|CastToBP_AICarExample OtherActor))
    (switch Utilities|FlowControl|Switch|SwitchonETriggerType (Variables|AIConfig|GetTriggerType)
      (:NewEnumerator0
        (Variables|TriggerBoxVars|SetTriggeredCar 0))
      (:NewEnumerator2
        (Variables|/Game/BP_BlueprintDublicates/BP_AICarExample.BP_AICarExample_C|SetIsOnCrossRoad _asbp_aicar_example false)
        (Default|SetDefaultLeftTrace _asbp_aicar_example)
        (Variables|/Game/BP_BlueprintDublicates/BP_AICarExample.BP_AICarExample_C|SetIsOnMainDirection _asbp_aicar_example false)
        (Default|SetDefaultStates _asbp_aicar_example)))))

(fn ConstructionScript)

(fn SetLetPassCrossRoads
  (params (CanPassCrossRoads :type Boolean))
  (bind _triggeredcar (Variables|TriggerBoxVars|GetTriggeredCar))
  (Variables|TriggerBoxVars|SetLetPassCrossRoads CanPassCrossRoads)
  (if (Utilities|IsValid _triggeredcar)
    (Variables|/Game/BP_BlueprintDublicates/BP_AICarExample.BP_AICarExample_C|SetCanMove _triggeredcar (Variables|TriggerBoxVars|GetLetPassCrossRoads))
    (Default|SetDefaultLeftTrace _triggeredcar)))

(fn ResetOccupied
  (Variables|TriggerBoxVars|SetOccupied false))