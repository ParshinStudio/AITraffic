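; AI car traffic light variant with an arm that adds a secondary set of red, yellow and green lights.
; It overrides the parent's light-switching events, calls the parent, then toggles the secondary light components' visibility.
; Secondary green shows only in the Green state; Red, Pedestrians and Delay all show secondary red, while yellow follows its own on/off event.
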(event EventSwitchMainLights
  (params (NewLightState :type ELightState%20Enum :default "NewEnumerator0"))
  (bind _greenlightsecondary (Variables|Default|GetGreenLightSecondary))
  (bind _redlightsecondary (Variables|Default|GetRedLightSecondary))
  (|CallParentFunction NewLightState)
  (switch Utilities|FlowControl|Switch|SwitchonELightState NewLightState
    (:NewEnumerator0
      (Rendering|SetVisibility _greenlightsecondary true false)
      (Rendering|SetVisibility _redlightsecondary false false))
    (:NewEnumerator1
      (Rendering|SetVisibility _greenlightsecondary false false :!label _label)
      (Rendering|SetVisibility _redlightsecondary true false))
    (:NewEnumerator2
      (goto _label))
    (:NewEnumerator3
      (goto _label))))

(event EventSwitchYellowLight
  (params (SwitchOn :type Boolean))
  (|CallParentFunction SwitchOn)
  (Rendering|SetVisibility (Variables|Default|GetYellowLightSecondary) SwitchOn false))

(fn ConstructionScript)