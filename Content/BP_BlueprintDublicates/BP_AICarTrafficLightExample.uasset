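; Example traffic light for AI cars, where a parent light runs the intersection's signal cycle and drives its child lights.
; ChangeLightState re-arms timers through green, red and optional pedestrian phases, with optional delay states between them.
; Children mirror or oppose the parent by direction, except in shared pedestrian and delay phases.
; Each light applies changes after a timer, showing yellow around green, then updates lamp visibility, car trigger boxes and pedestrian lights.
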(event EventBeginPlay
  (for _array_element (Variables|TrafficConfig|GetLightTriggerBoxes)
    (Variables|/Game/BP_BlueprintDublicates/BP_AICarTriggerVolumeExample.BP_AICarTriggerVolumeExample_C|SetGreenLightTimer _array_element (Variables|TrafficConfig|GetGreenLightTime))
    (Variables|/Game/BP_BlueprintDublicates/BP_AICarTriggerVolumeExample.BP_AICarTriggerVolumeExample_C|SetIsMainDirection _array_element (Variables|TrafficConfig|GetIsMainDirection)))
  (if (Variables|TrafficConfig|GetIsParentLight)
    (for _array_element_2 (Variables|TrafficConfig|GetChildrenLights)
      (Variables|BP_AICarTrafficLightExample_C|SetYellowActiveTimer _array_element_2 (Variables|TrafficConfig|GetYellowActiveTimer)))
    (CallFunction|ChangeLightState)))

(fn ConstructionScript)

(fn ChangeLightState
  (bind _delayafterred (Variables|TrafficConfig|GetDelayAfterRed))
  (bind _returnvalue (!= _delayafterred 0.0))
  (switch Utilities|FlowControl|Switch|SwitchonELightState (Variables|Default|GetLightState)
    (:NewEnumerator0
      (if (!= (Variables|TrafficConfig|GetDelayAfterGreen) 0.0)
        (CallFunction|SetDelayState)
        (bind _returnvalue_2 (Utilities|Time|SetTimerbyFunctionName self "ChangeLightState" 1.0 false (- (Variables|TrafficConfig|GetDelayAfterGreen) (Variables|TrafficConfig|GetYellowActiveTimer))))
        (Variables|Default|SetMainLightSwitchHandle _returnvalue_2)
        (Variables|Default|SetPreviousLightState "NewEnumerator0")
        (else
          (CallFunction|SetRedState :!label _label)
          (bind _returnvalue_3 (Utilities|Time|SetTimerbyFunctionName self "ChangeLightState" 1.0 false (- (Variables|TrafficConfig|GetRedLightTime) (Variables|TrafficConfig|GetYellowActiveTimer))))
          (Variables|Default|SetMainLightSwitchHandle _returnvalue_3))))
    (:NewEnumerator1
      (if (== (Variables|TrafficConfig|GetPedestriansTime) 0.0)
        (if _returnvalue
          (CallFunction|SetDelayState :!label _label_2)
          (bind _returnvalue_4 (Utilities|Time|SetTimerbyFunctionName self "ChangeLightState" 1.0 false (- (Variables|TrafficConfig|GetDelayAfterRed) (Variables|TrafficConfig|GetYellowActiveTimer))))
          (Variables|Default|SetMainLightSwitchHandle _returnvalue_4)
          (Variables|Default|SetPreviousLightState "NewEnumerator1")
          (else
            (CallFunction|SetGreenState :!label _label_3)
            (bind _returnvalue_5 (Utilities|Time|SetTimerbyFunctionName self "ChangeLightState" 1.0 false (- (Variables|TrafficConfig|GetGreenLightTime) (Variables|TrafficConfig|GetYellowActiveTimer))))
            (Variables|Default|SetMainLightSwitchHandle _returnvalue_5)))
        (elif _returnvalue
          (goto _label_2)
          (else
            (CallFunction|SetPedestriansState :!label _label_4)
            (bind _returnvalue_6 (Utilities|Time|SetTimerbyFunctionName self "ChangeLightState" 1.0 false (- (Variables|TrafficConfig|GetPedestriansTime) (Variables|TrafficConfig|GetYellowActiveTimer))))
            (Variables|Default|SetMainLightSwitchHandle _returnvalue_6)))))
    (:NewEnumerator2
      (if (!= (Variables|TrafficConfig|GetDelayAfterPedestrians) 0.0)
        (CallFunction|SetDelayState)
        (bind _returnvalue_7 (Utilities|Time|SetTimerbyFunctionName self "ChangeLightState" 1.0 false (- (Variables|TrafficConfig|GetDelayAfterPedestrians) (Variables|TrafficConfig|GetYellowActiveTimer))))
        (Variables|Default|SetMainLightSwitchHandle _returnvalue_7)
        (Variables|Default|SetPreviousLightState "NewEnumerator2")
        (else
          (goto _label_3))))
    (:NewEnumerator3
      (switch Utilities|FlowControl|Switch|SwitchonELightState (Variables|Default|GetPreviousLightState)
        (:NewEnumerator0
          (goto _label))
        (:NewEnumerator1
          (if (== (Variables|TrafficConfig|GetPedestriansTime) 0.0)
            (goto _label_3)
            (else
              (goto _label_4))))
        (:NewEnumerator2
          (goto _label_3))))))

(fn SetGreenState
  (CallFunction|SetLightCondition "NewEnumerator0")
  (for _array_element (Variables|TrafficConfig|GetChildrenLights)
    (if (Variables|BP_AICarTrafficLightExample_C|GetIsInSameDirection _array_element)
      (CallFunction|SetLightCondition _array_element "NewEnumerator0")
      (else
        (CallFunction|SetLightCondition _array_element "NewEnumerator1")))))

(fn SetRedState
  (CallFunction|SetLightCondition "NewEnumerator1")
  (for _array_element (Variables|TrafficConfig|GetChildrenLights)
    (if (Variables|BP_AICarTrafficLightExample_C|GetIsInSameDirection _array_element)
      (CallFunction|SetLightCondition _array_element "NewEnumerator1")
      (else
        (CallFunction|SetLightCondition _array_element "NewEnumerator0")))))

(fn SetPedestriansState
  (CallFunction|SetLightCondition "NewEnumerator2")
  (for _array_element (Variables|TrafficConfig|GetChildrenLights)
    (CallFunction|SetLightCondition _array_element "NewEnumerator2")))

(fn SetDelayState
  (CallFunction|SetLightCondition "NewEnumerator3")
  (for _array_element (Variables|TrafficConfig|GetChildrenLights)
    (CallFunction|SetLightCondition _array_element "NewEnumerator3")))

(fn SetLightCondition
  (params (NewLightState :type ELightState%20Enum :default "NewEnumerator0"))
  (if (or (Utilities|Enum|Equal(Enum) (Variables|Default|GetLightState) "NewEnumerator0") (Utilities|Enum|Equal(Enum) NewLightState "NewEnumerator0"))
    (Variables|Default|SetYellowLightState true)
    (CallFunction|SwitchYellowLight true))
  (Variables|Default|SetLightState NewLightState)
  (bind _returnvalue (Utilities|Time|SetTimerbyFunctionName self "SetLightConditionResume" 1.0 false (Variables|TrafficConfig|GetYellowActiveTimer)))
  (Variables|Default|SetYellowLightDelayHandle _returnvalue))

(fn SetLightConditionResume
  (bind _lighttriggerboxes (Variables|TrafficConfig|GetLightTriggerBoxes))
  (bind _pedestrianlights (Variables|TrafficConfig|GetPedestrianLights))
  (CallFunction|SwitchMainLights (Variables|Default|GetLightState))
  (if (Variables|Default|GetYellowLightState)
    (Variables|Default|SetYellowLightState false)
    (CallFunction|SwitchYellowLight false))
  (if (!= (Utilities|Array|Length (Variables|TrafficConfig|GetLightTriggerBoxes)) 0)
    (if (Utilities|Enum|Equal(Enum) (Variables|Default|GetLightState) "NewEnumerator0")
      (for _array_element _lighttriggerboxes
        (Default|SetLetPassCrossRoads _array_element true))
      (else
        (for _array_element_2 _lighttriggerboxes
          (Default|SetLetPassCrossRoads _array_element_2 false)))))
  (if (!= (Utilities|Array|Length (Variables|TrafficConfig|GetPedestrianLights)) 0)
    (if (Utilities|Enum|Equal(Enum) (Variables|Default|GetLightState) "NewEnumerator2")
      (for _array_element_3 _pedestrianlights
        (Default|SetPedestrianLightState _array_element_3 true))
      (else
        (for _array_element_4 _pedestrianlights
          (Default|SetPedestrianLightState _array_element_4 false))))))

(fn SwitchMainLights
  (params (NewLightState :type ELightState%20Enum :default "NewEnumerator0"))
  (bind _redlightprimary (Variables|Default|GetRedLightPrimary))
  (bind _greenlightprimary (Variables|Default|GetGreenLightPrimary))
  (switch Utilities|FlowControl|Switch|SwitchonELightState NewLightState
    (:NewEnumerator0
      (Rendering|SetVisibility _greenlightprimary true false)
      (Rendering|SetVisibility _redlightprimary false false))
    (:NewEnumerator1
      (Rendering|SetVisibility _greenlightprimary false false :!label _label)
      (Rendering|SetVisibility _redlightprimary true false))
    (:NewEnumerator2
      (goto _label))
    (:NewEnumerator3
      (goto _label))))

(fn SwitchYellowLight
  (params (SwitchOn :type Boolean))
  (Rendering|SetVisibility (Variables|Default|GetYellowLightPrimary) SwitchOn false))