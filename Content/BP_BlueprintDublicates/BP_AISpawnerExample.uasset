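; AI traffic spawner that maintains a randomized number of BP_AICarExample cars around the player.
; CarsSpawner runs on BeginPlay; the looping timer names "CarSpawner", which doesn't match that function.
; Each pass destroys distant cars, then gathers nearby spawn points, requiring an unblocked player-to-point visibility trace at mid range.
; It spawns missing cars at random unique points, snapped to each point's spline, which it assigns to the car.
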(event EventBeginPlay
  (bind _carspawnrate (Variables|AIConfig|GetCarSpawnRate))
  (CallFunction|CarsSpawner)
  (bind _returnvalue (Utilities|Time|SetTimerbyFunctionName self "CarSpawner" _carspawnrate true _carspawnrate))
  (Variables|SpawnerVars|SetCarSpawnerHandle _returnvalue))

(fn ConstructionScript)

(fn CarsSpawner
  (bind _traceblockspawndistance (Variables|AIConfig|GetTraceBlockSpawnDistance))
  (bind _foundcars (Variables|SpawnerVars|GetFoundCars))
  (bind _nearbycarspawnpoints (Variables|SpawnerVars|GetNearbyCarSpawnPoints))
  (bind _mincarsaround (Variables|AIConfig|GetMinCarsAround))
  (bind _nearbycarspawnpoints_2 (Variables|SpawnerVars|GetNearbyCarSpawnPoints))
  (bind _maxcarsaround (Variables|AIConfig|GetMaxCarsAround))
  (bind _returnvalue (Utilities|Array|Length _foundcars))
  (bind _returnvalue_2 (Utilities|Array|Length _nearbycarspawnpoints))
  (bind _returnvalue_3 (Math|Random|RandomIntegerinRange _mincarsaround _maxcarsaround))
  (Variables|SpawnerVars|SetPlayerLocation (Transformation|GetActorLocation (Game|Player|GetPlayerPawn 0)))
  (bind _outactors (Actor|GetAllActorsOfClass "/Game/BP_BlueprintDublicates/BP_AICarExample.BP_AICarExample_C"))
  (for _array_element _outactors
    (if (> (Math|Vector|Distance(Vector) (Variables|SpawnerVars|GetPlayerLocation) (Transformation|GetActorLocation _array_element)) (Variables|AIConfig|GetDestructorDistance))
      (Actor|DestroyActor _array_element)
      (else
        (Utilities|Array|Add (Variables|SpawnerVars|GetFoundCars) 0))))
  (if (> _returnvalue_3 _returnvalue)
    (Variables|SpawnerVars|SetCarsToSpawn (- _returnvalue_3 _returnvalue))
    (bind _outactors_2 (Collision|SphereOverlapActors (Variables|SpawnerVars|GetPlayerLocation) (Variables|AIConfig|GetMaxSpawnDistance) (Variables|AIConfig|GetTraceCollisionResponse) "/Game/BP_BlueprintDublicates/BP_AICarSpawnPointExample.BP_AICarSpawnPointExample_C"))
    (for _array_element_2 _outactors_2
      (if (and (> (Math|Vector|Distance(Vector) (Variables|SpawnerVars|GetPlayerLocation) (Transformation|GetActorLocation _array_element_2)) (Variables|AIConfig|GetMinSpawnDistance)) (< (Math|Vector|Distance(Vector) (Variables|SpawnerVars|GetPlayerLocation) (Transformation|GetActorLocation _array_element_2)) _traceblockspawndistance))
        (bind _outhit (Collision|LineTraceByChannel (Variables|SpawnerVars|GetPlayerLocation) (Transformation|GetActorLocation _array_element_2) "TraceTypeQuery1" false 0 "None"))
        (if (not (.bBlockingHit (Collision|BreakHitResult _outhit)))
          (Utilities|Array|Add (Variables|SpawnerVars|GetNearbyCarSpawnPoints) _array_element_2))
        (elif (> (Math|Vector|Distance(Vector) (Variables|SpawnerVars|GetPlayerLocation) (Transformation|GetActorLocation _array_element_2)) _traceblockspawndistance)
          (Utilities|Array|Add (Variables|SpawnerVars|GetNearbyCarSpawnPoints) _array_element_2))))
    (if (> _returnvalue_2 0)
      (if (> (Variables|SpawnerVars|GetCarsToSpawn) _returnvalue_2)
        (Variables|SpawnerVars|SetCarsToSpawn _returnvalue_2)
        (else
          (Variables|SpawnerVars|SetCarsToSpawn (Variables|SpawnerVars|GetCarsToSpawn))))
      (for _index (range 0 (- (Variables|SpawnerVars|GetCarsToSpawn) 1))
        (while (or (not (Utilities|IsValid (Variables|SpawnerVars|GetCarSpawnPoint))) (Utilities|Array|ContainsItem (Variables|SpawnerVars|GetUsedCarSpawnPoints) (Variables|SpawnerVars|GetCarSpawnPoint)))
          (Variables|SpawnerVars|SetCarSpawnPoint (Utilities|Array|Get(acopy) _nearbycarspawnpoints_2 (Math|Random|RandomIntegerinRange 0 (- (Utilities|Array|Length _nearbycarspawnpoints_2) 1)))))
        (Utilities|Array|Add (Variables|SpawnerVars|GetUsedCarSpawnPoints) (Variables|SpawnerVars|GetCarSpawnPoint))
        (bind _asbp_aicar_spawn_point_example (Utilities|Casting|CastToBP_AICarSpawnPointExample (Variables|SpawnerVars|GetCarSpawnPoint)))
        (if (Utilities|IsValid (Variables|/Game/BP_BlueprintDublicates/BP_AICarSpawnPointExample.BP_AICarSpawnPointExample_C|GetSpawnSpline _asbp_aicar_spawn_point_example))
          (bind _returnvalue_4 (Game|SpawnActorfromClass "/Game/BP_BlueprintDublicates/BP_AICarExample.BP_AICarExample_C" (Math|Transform|MakeTransform (Spline|FindLocationClosesttoWorldLocation (Variables|/Game/BP_BlueprintDublicates/BP_AICarSplineExample.BP_AICarSplineExample_C|GetSplineComponent (Variables|/Game/BP_BlueprintDublicates/BP_AICarSpawnPointExample.BP_AICarSpawnPointExample_C|GetSpawnSpline _asbp_aicar_spawn_point_example)) (Transformation|GetActorLocation _asbp_aicar_spawn_point_example) "World") (Class|SplineComponent|FindRotationClosesttoWorldLocation (Variables|/Game/BP_BlueprintDublicates/BP_AICarSplineExample.BP_AICarSplineExample_C|GetSplineComponent (Variables|/Game/BP_BlueprintDublicates/BP_AICarSpawnPointExample.BP_AICarSpawnPointExample_C|GetSpawnSpline _asbp_aicar_spawn_point_example)) (Spline|FindLocationClosesttoWorldLocation (Variables|/Game/BP_BlueprintDublicates/BP_AICarSplineExample.BP_AICarSplineExample_C|GetSplineComponent (Variables|/Game/BP_BlueprintDublicates/BP_AICarSpawnPointExample.BP_AICarSpawnPointExample_C|GetSpawnSpline _asbp_aicar_spawn_point_example)) (Transformation|GetActorLocation _asbp_aicar_spawn_point_example) "World") "World") "1,1,1") "DontSpawnIfColliding" 0 0))
          (if (Utilities|IsValid _returnvalue_4)
            (Default|SetNewSpline _returnvalue_4 (Variables|/Game/BP_BlueprintDublicates/BP_AICarSpawnPointExample.BP_AICarSpawnPointExample_C|GetSpawnSpline _asbp_aicar_spawn_point_example)))))
      (CallFunction|EmptyArrays)
      (else
        (CallFunction|EmptyArrays)))
    (else
      (CallFunction|EmptyArrays))))

(fn EmptyArrays
  (Utilities|Array|Clear (Variables|SpawnerVars|GetFoundCars))
  (Utilities|Array|Clear (Variables|SpawnerVars|GetNearbyCarSpawnPoints))
  (Utilities|Array|Clear (Variables|SpawnerVars|GetUsedCarSpawnPoints))
  (Variables|SpawnerVars|SetCarSpawnPoint 0))